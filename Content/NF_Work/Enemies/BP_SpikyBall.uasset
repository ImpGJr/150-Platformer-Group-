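; BP_SpikyBall is an enemy spiky ball that moves along its local X axis, pitching in 90-degree steps to follow surfaces.
; Each Tick, a forward trace hit pitches it +90; otherwise a second trace, offset by scaled negated actor location, gates swept movement.
; When that trace misses, IsTurning delays the -90 pitch by one tick.
; The construction script tints the mesh through a dynamic material.
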(event `self.ReceiveTick`
  (params (DeltaSeconds :type "Float (single-precision)"))
  (set `self.Delta Seconds` DeltaSeconds)
  (`|ExecutionSequence`
    (:`then_0`
      (bind (_outhit _returnvalue) (`KismetSystemLibrary.LineTraceSingle` (`self.K2_GetActorLocation`) (+ (`self.K2_GetActorLocation`) (* (`self.GetActorForwardVector`) (`self.BlockDistance`))) "TraceTypeQuery1"))
      (if _returnvalue
        (`self.K2_AddActorLocalRotation` (`KismetMathLibrary.MakeRotator` 0.0 90.0))
        (else
          (bind (_outhit_2 _returnvalue_2) (`KismetSystemLibrary.LineTraceSingle` (`self.K2_GetActorLocation`) (+ (`self.K2_GetActorLocation`) (* (`self.K2_GetActorLocation`) -1.0 (`self.DownwardDistance`))) "TraceTypeQuery1"))
          (if _returnvalue_2
            (set `self.IsTurning` false)
            (`self.K2_AddActorLocalOffset` (`KismetMathLibrary.MakeVector` (* (`self.MoveSpeed`) (`self.Delta Seconds`))) true)
            (elif (`self.IsTurning`)
              (`self.K2_AddActorLocalRotation` (`KismetMathLibrary.MakeRotator` 0.0 -90.0))
              (else
                (set `self.IsTurning` true)))))))
    (:`then_1`
      (`KismetSystemLibrary.LineTraceSingle` (0.0 0.0 0.0) (0.0 0.0 0.0) "TraceTypeQuery1"))))

(fn `UserConstructionScript`
  (bind _returnvalue (`PrimitiveComponent.CreateDynamicMaterialInstance` (`self.SpikyBall`) 0 null "None"))
  (`MaterialInstanceDynamic.SetVectorParameterValue` _returnvalue "Color" (`self.Value`)))