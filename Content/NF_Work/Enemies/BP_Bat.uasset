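; BP_Bat is a bat enemy that hangs until BP_CubeMcCubey enters its Detection volume, then attacks.
; Tick runs a Hanging, Swooping, Chasing, Returning state machine through movement input, swooping to the player's captured position, chasing, then returning home once the player is out of close range.
; The chase's sine wobble is multiplied to zero, projectile hits subtract zero health, and player damage logic is unconnected.
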(event `self.ReceiveBeginPlay`
  ; Set health and location
  (set `self.Location` (`self.K2_GetActorLocation`))
  (set `self.Health` 50))

(event `self.Detection.OnComponentBeginOverlap`
  (params (OverlappedComponent :type "PrimitiveComponent Object Reference") (OtherActor :type "Actor Object Reference") (OtherComp :type "PrimitiveComponent Object Reference") (OtherBodyIndex :type Integer) (bFromSweep :type Boolean) (SweepResult :type "HitResult Structure (by ref)"))
  ; Player taking damage
  (bind _asbp_cube_mc_cubey (cast `/Game/Blueprints/Character/BP_CubeMcCubey` OtherActor))
  (set `self.TargetPlayer ` _asbp_cube_mc_cubey)
  (if (`|EnumEquality` (`self.CurrentState`) "NewEnumerator0")
    (set `self.SwoopLocation` (`self.K2_GetActorLocation` (`self.TargetPlayer `)))
    (set `self.CurrentState` "NewEnumerator1")))

(event `self.Hitbox.OnComponentBeginOverlap`
  (params (OverlappedComponent :type "PrimitiveComponent Object Reference") (OtherActor :type "Actor Object Reference") (OtherComp :type "PrimitiveComponent Object Reference") (OtherBodyIndex :type Integer) (bFromSweep :type Boolean) (SweepResult :type "HitResult Structure (by ref)"))
  ; taking damage
  (cast `/Game/Blueprints/Projectiles/BP_Player_Projectile` OtherActor)
  (set `self.Health` (- (`self.Health`) 0)))

(event `self.ReceiveTick`
  (params (DeltaSeconds :type "Float (single-precision)"))
  ; Bat movement
  (switch `/Game/NF_Work/Enemies/Enum_EnemyState` (`self.CurrentState`)
    (:`NewEnumerator1`
      (`self.AddMovementInput` (`KismetMathLibrary.Normal` (- (`self.SwoopLocation`) (`self.K2_GetActorLocation`))))
      (if (< (`KismetMathLibrary.Vector_Distance` (`self.K2_GetActorLocation`) (`self.SwoopLocation`)) 50.0)
        (set `self.CurrentState` "NewEnumerator2")))
    (:`NewEnumerator2`
      (`self.AddMovementInput` (+ (`KismetMathLibrary.Normal` (- (`self.K2_GetActorLocation` (`self.TargetPlayer `)) (`self.K2_GetActorLocation`))) (`KismetMathLibrary.MakeVector` 0.0 0.0 (* (* 0.0 (`KismetMathLibrary.DegSin` (* (`KismetSystemLibrary.GetGameTimeInSeconds`) 6.0)) (`self.Wave`)) 0.6))) 1.0 true)
      (if (> (`KismetMathLibrary.Vector_Distance` (`self.K2_GetActorLocation`) (`self.K2_GetActorLocation` (`self.TargetPlayer `))) 100.0)
        (set `self.CurrentState` "NewEnumerator3")))
    (:`NewEnumerator3`
      (`self.AddMovementInput` (`KismetMathLibrary.Normal` (- (`self.Location`) (`self.K2_GetActorLocation`))) 8.0)
      (if (< (`KismetMathLibrary.Vector_Distance` (`self.K2_GetActorLocation`) (`self.Location`)) 25.0)
        (set `self.Location` (`self.K2_GetActorLocation`))
        (`MovementComponent.StopMovementImmediately` (`self.FloatingPawnMovement`))
        (set `self.CurrentState` "NewEnumerator0")))))

(fn `UserConstructionScript`)